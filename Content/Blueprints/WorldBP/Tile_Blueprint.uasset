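; Tile actor that shows whether it is Movable or Non-Movable through a tinted material overlay.
; On BeginPlay it creates a dynamic material instance from the overlay material on its render component, then calls SetMaterialColor.
; SetMaterialColor switches on TileType to set the overlay color and alpha parameters, leaving Movable tiles semi-opaque and Non-Movable overlays fully transparent.
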(event EventBeginPlay
  (bind _returnvalue (Rendering|Material|CreateDynamicMaterialInstance (Variables|Default|GetRenderComponent) 0 "/Game/Materials/TileOverlayMat.TileOverlayMat" "MaterialInstance" :!class /Script/Engine.PrimitiveComponent))
  (Variables|Default|SetDynamicMaterialInstance _returnvalue)
  (CallFunction|SetMaterialColor))

(event Collision|EventActorBeginOverlap
  (params (OtherActor :type Actor%20Object%20Reference)))

(event EventTick
  (params (DeltaSeconds :type Float%20%28single-precision%29)))

(fn ConstructionScript)

(fn SetMaterialColor
  (bind _dynamicmaterialinstance (Variables|Default|GetDynamicMaterialInstance))
  (switch Utilities|FlowControl|Switch|SwitchonTileType (Variables|Default|GetTileType)
    (:NewEnumerator0
      (Rendering|Material|SetVectorParameterValue _dynamicmaterialinstance "TileOverlayColor" (Variables|Default|GetMovableColor) :!class /Script/Engine.MaterialInstanceDynamic)
      (Rendering|Material|SetScalarParameterValue (Variables|Default|GetDynamicMaterialInstance) "TileOverlayAlpha" 0.6 :!class /Script/Engine.MaterialInstanceDynamic))
    (:NewEnumerator1
      (Rendering|Material|SetVectorParameterValue _dynamicmaterialinstance "TileOverlayColor" (Variables|Default|GetNonMovableColor) :!class /Script/Engine.MaterialInstanceDynamic)
      (Rendering|Material|SetScalarParameterValue _dynamicmaterialinstance "TileOverlayAlpha" 0.0 :!class /Script/Engine.MaterialInstanceDynamic))))