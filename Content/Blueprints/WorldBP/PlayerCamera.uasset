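; PlayerCamera is a player camera Blueprint that pans across the world's XY plane as the player drags a finger.
; Pressing Touch1 records the start and previous screen locations.
; While the touch is held, Tick converts the screen delta since the last move into an unscaled, axis-swapped world offset without sweep.
; Movement applies only while the finger is at least a small pixel threshold from its start point, filtering out taps.
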(event EventTick
  (params (DeltaSeconds :type Float%20%28single-precision%29))
  (bind _returnvalue (Game|GetPlayerController 0))
  (bind (_locationx _locationy _biscurrentlypressed) (Class|PlayerController|GetInputTouchState _returnvalue "Touch1"))
  (if _biscurrentlypressed
    (Variables|Default|SetCurrentTouchLocation (Math|Vector2D|MakeVector2D _locationx _locationy))
    (if (>= (Math|Vector2D|Vector2DLength (- (Variables|Default|GetCurrentTouchLocation) (Variables|Default|GetFirstTouchLocation))) 1e+01)
      (Transformation|AddActorWorldOffset (Math|Vector|MakeVector (.y (- (Variables|Default|GetCurrentTouchLocation) (Variables|Default|GetPreviousTouchLocation))) (* (.x (- (Variables|Default|GetCurrentTouchLocation) (Variables|Default|GetPreviousTouchLocation))) -1.0) 0.0))
      (Variables|Default|SetPreviousTouchLocation (Variables|Default|GetCurrentTouchLocation)))))

(event Input|TouchEvents|Touch1
  (params (Key :type Key%20Structure :default "None"))
  (bind _returnvalue (Game|GetPlayerController 0))
  (bind (_locationx _locationy) (Class|PlayerController|GetInputTouchState _returnvalue "Touch1"))
  (:Pressed
    (bind _output_get (Variables|Default|SetPreviousTouchLocation (Math|Vector2D|MakeVector2D _locationx _locationy)))
    (Variables|Default|SetFirstTouchLocation _output_get)))

(fn ConstructionScript)