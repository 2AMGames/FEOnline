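; TileManager spawns a fixed-size square grid of Tile_Blueprint actors when play begins.
; BeginPlay finds the minimum X/Y corner of the referenced actor's (NewVar0) brush bounds, insets it by SpriteSize and passes it to CreateTiles at a fixed height.
; CreateTiles clears the Tiles array, spawns rotated tiles in nested loops spaced by Offset, stores each one, then prints a completion message.
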(event EventBeginPlay
  (bind _newvar_0 (Variables|Default|GetNewVar_0))
  (bind _spritesize (Variables|Default|GetSpriteSize))
  (bind _returnvalue (Actor|GetComponentsByClass _newvar_0 "/Script/Engine.BrushComponent"))
  (bind _output (Utilities|Array|Get(acopy) _returnvalue))
  (bind (_origin _boxextent) (Collision|GetComponentBounds _output))
  (CallFunction|CreateTiles (Math|Vector|MakeVector (+ (- (.x _origin) (.x _boxextent)) _spritesize) (+ (- (.y _origin) (.y _boxextent)) _spritesize) 112.0) "(X=10.000000,Y=10.000000)"))

(fn ConstructionScript)

(fn CreateTiles
  (params (BottomLeft_Corner :type Vector) (Dimensions :type Vector%202D%20Structure))
  (bind _offset (LocalVariables|GetOffset))
  (Utilities|Array|Clear (Variables|Default|GetTiles))
  (while (< (LocalVariables|GetxDimension) (Math|Float|Truncate (.x Dimensions)))
    (LocalVariables|SetyDimension 0)
    (while (< (LocalVariables|GetyDimension) (Math|Float|Truncate (.y Dimensions)))
      (bind _returnvalue (Game|SpawnActorfromClass "/Game/Blueprints/WorldBP/Tile_Blueprint.Tile_Blueprint_C" (Math|Transform|MakeTransform (Math|Vector|MakeVector (+ (* (Math|Float|Truncate (Math|Conversions|ToFloat(Integer) (LocalVariables|GetxDimension))) _offset) (.x BottomLeft_Corner)) (+ (.y BottomLeft_Corner) (* (LocalVariables|GetyDimension) _offset)) (.z BottomLeft_Corner)) "0, 0,-90.000000" "1,1,1") "Undefined" 0 0))
      (Utilities|Array|Add (Variables|Default|GetTiles) _returnvalue)
      (LocalVariables|SetyDimension (+ (LocalVariables|GetyDimension) 1)))
    (LocalVariables|SetxDimension (+ (LocalVariables|GetxDimension) 1)))
  (Development|PrintString "\"Finished\"" true true "(R=0.000000,G=0.660000,B=1.000000,A=1.000000)" 12.0))